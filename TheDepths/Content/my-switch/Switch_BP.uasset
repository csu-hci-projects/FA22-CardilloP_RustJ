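; A grabbable breaker switch that controls the tagged Roof, Monitor and Radio point lights.
; Tick turns the Handle's clamped roll by the X offset between Arrow and Grabbed, and dropping snaps Grabbed back to the Handle.
; Near full throw, lights turn on with a sound only if no "FIxable" actors remain; otherwise the handle resets after a delay.
; Below that threshold the lights are off; an older MotionController look-at path is unconnected.
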(event `self.ReceiveTick`
  (params (DeltaSeconds :type "Float (single-precision)"))
  (bind _handle (`self.Handle`))
  (bind (_returnvalue_roll _returnvalue_pitch _returnvalue_yaw) (`KismetMathLibrary.BreakRotator` (`SceneComponent.K2_GetComponentRotation` _handle)))
  (bind _returnvalue_roll_2 (`KismetMathLibrary.BreakRotator` (`SceneComponent.K2_GetComponentRotation` (`self.Handle`))))
  (bind _returnvalue_x (`KismetMathLibrary.BreakVector` (- (`SceneComponent.K2_GetComponentLocation` (`self.Arrow`)) (`SceneComponent.K2_GetComponentLocation` (`self.grabbed`)))))
  (`SceneComponent.K2_SetWorldRotation` _handle (`KismetMathLibrary.MakeRotator` (`KismetMathLibrary.FClamp` (+ _returnvalue_roll _returnvalue_x) 0.0 180.0) _returnvalue_pitch _returnvalue_yaw) false false)
  (if (<= _returnvalue_roll_2 177.0)
    (bind _outactors (`GameplayStatics.GetAllActorsOfClassWithTag` "/Script/Engine.PointLight" "Roof"))
    (for _array_element _outactors
      (`LightComponent.SetIntensity` (`PointLight.PointLightComponent` _array_element) 0.0))
    (bind _outactors_2 (`GameplayStatics.GetAllActorsOfClassWithTag` "/Script/Engine.PointLight" "Monitor"))
    (for _array_element_2 _outactors_2
      (`LightComponent.SetIntensity` (`PointLight.PointLightComponent` _array_element_2) 0.0))
    (bind _outactors_3 (`GameplayStatics.GetAllActorsOfClassWithTag` "/Script/Engine.PointLight" "Radio"))
    (for _array_element_3 _outactors_3
      (`LightComponent.SetIntensity` (`PointLight.PointLightComponent` _array_element_3) 0.0)
      (set `self.flipped` true))
    (else
      (bind _outactors_4 (`GameplayStatics.GetAllActorsWithTag` "FIxable"))
      (if (== 0 (`KismetArrayLibrary.Array_Length` _outactors_4))
        (if (`self.flipped`)
          (`GameplayStatics.PlaySoundAtLocation` "/Game/Sounds/131599__echocinematics__kill-switch-large-breaker-switch.131599__echocinematics__kill-switch-large-breaker-switch" (`SceneComponent.K2_GetComponentLocation` (`self.Handle`)) (struct) 1.0 1.0 0.0 null null null null)
          (set `self.flipped` false))
        (bind _outactors_5 (`GameplayStatics.GetAllActorsOfClassWithTag` "/Script/Engine.PointLight" "Roof"))
        (for _array_element_4 _outactors_5
          (`LightComponent.SetIntensity` (`PointLight.PointLightComponent` _array_element_4) 0.3))
        (bind _outactors_6 (`GameplayStatics.GetAllActorsOfClassWithTag` "/Script/Engine.PointLight" "Monitor"))
        (for _array_element_5 _outactors_6
          (`LightComponent.SetIntensity` (`PointLight.PointLightComponent` _array_element_5) 0.1))
        (bind _outactors_7 (`GameplayStatics.GetAllActorsOfClassWithTag` "/Script/Engine.PointLight" "Radio"))
        (for _array_element_6 _outactors_7
          (`LightComponent.SetIntensity` (`PointLight.PointLightComponent` _array_element_6) 0.01))
        (else
          (`KismetSystemLibrary.Delay` 5.0)
          (`SceneComponent.K2_SetWorldRotation` :`self` (`self.Handle`))
          (`SceneComponent.K2_SetRelativeLocationAndRotation` (`self.grabbed`) (`SceneComponent.K2_GetComponentLocation` (`self.Handle`)) (`SceneComponent.K2_GetComponentRotation` (`self.Handle`)) false false))))))

(event `self.GrabComponent1.OnDropped`
  (`SceneComponent.K2_SetRelativeLocationAndRotation` (`self.grabbed`) (`SceneComponent.K2_GetComponentLocation` (`self.Handle`)) (`SceneComponent.K2_GetComponentRotation` (`self.Handle`)) false false))

(fn `UserConstructionScript`)